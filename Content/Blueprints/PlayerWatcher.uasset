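; PlayerWatcher is an actor that turns its Scene component to keep facing the first-person player.
; BeginPlay caches the BP_FirstPersonCharacter reference.
; Each Tick takes the arccosine of the dot between the forward vector and the player direction, using the right-vector dot's sign to extend it to 360 degrees.
; The result sets only relative yaw, though the angle uses the full 3D direction, so height differences affect it.
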(event EventBeginPlay
  (bind _returnvalue (Actor|GetActorOfClass "/Game/FirstPerson/Blueprints/BP_FirstPersonCharacter.BP_FirstPersonCharacter_C"))
  (Variables|Default|SetPlayerRef _returnvalue))

(event EventTick
  (params (DeltaSeconds :type Float%20%28single-precision%29))
  (bind _returnvalue (Transformation|GetActorForwardVector))
  (bind _returnvalue_2 (Transformation|GetActorLocation))
  (bind _playerref (Variables|Default|GetPlayerRef))
  (bind _scene (Variables|Default|GetScene))
  (bind _returnvalue_3 (Math|Vector|Normalize _returnvalue))
  (bind _returnvalue_4 (Transformation|GetActorLocation _playerref))
  (bind _returnvalue_5 (- _returnvalue_4 _returnvalue_2))
  (bind _returnvalue_6 (Math|Vector|Normalize _returnvalue_5))
  (bind _returnvalue_7 (Math|Vector|DotProduct _returnvalue_6 _returnvalue_3))
  (bind _returnvalue_8 (Class|KismetMathLibrary|DegAcos _returnvalue_7))
  (if (< (Math|Vector|DotProduct (Math|Vector|Normalize (- (Transformation|GetActorLocation (Variables|Default|GetPlayerRef)) (Transformation|GetActorLocation (Components|GetOwner (Variables|Default|GetScene))))) (Math|Vector|Normalize (Transformation|GetActorRightVector))) 0.0)
    (Transformation|SetRelativeRotation _scene (Math|Rotator|MakeRotator 0.0 0.0 (- 3.6e+02 _returnvalue_8)) false false)
    (else
      (Transformation|SetRelativeRotation _scene (Math|Rotator|MakeRotator 0.0 0.0 _returnvalue_8) false false))))

(fn ConstructionScript)